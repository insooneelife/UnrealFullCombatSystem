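; DisplayedItemBP is an item actor in the Dynamic Combat System that represents an item displayed on its owning Character.
; It finds its primary component by preferring a static mesh, then a skeletal mesh, then a particle system, and disables that component's collision on BeginPlay.
; Attach parents this component to the owner's mesh at the attachment socket and reports success.
; SimulatePhysics switches it to the Ragdoll collision profile and enables physics.
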(event EventBeginPlay
  (bind _component (CallFunction|GetPrimaryComponent))
  (Utilities|IsValid _component
    (:Is%20Valid
      (Collision|SetCollisionEnabled _component "NoCollision"))))

(fn ConstructionScript)

(fn GetPrimaryComponent
  (bind _returnvalue (Actor|GetComponentbyClass "/Script/Engine.StaticMeshComponent"))
  (bind _returnvalue_2 (Actor|GetComponentbyClass "/Script/Engine.SkeletalMeshComponent"))
  (Utilities|IsValid _returnvalue
    (:Is%20Valid
      (return _returnvalue))
    (:Is%20Not%20Valid
      (Utilities|IsValid _returnvalue_2
        (:Is%20Valid
          (return _returnvalue_2))
        (:Is%20Not%20Valid
          (return (Actor|GetComponentbyClass "/Script/Engine.ParticleSystemComponent")))))))

(fn Attach
  (bind _output_get (LocalVariables|SetL_MeshComponent (CallFunction|GetPrimaryComponent)))
  (Utilities|IsValid _output_get
    (:Is%20Valid
      (Transformation|AttachComponentToComponent (LocalVariables|GetL_MeshComponent) (Variables|/Script/Engine.Character|GetMesh (.AsCharacter (Utilities|Casting|CastToCharacter (Components|GetOwner)))) (CallFunction|GetAttachmentSocket) "KeepRelative" "KeepRelative" "KeepRelative" false)
      (return true))
    (:Is%20Not%20Valid
      (return false))))

(fn GetAttachmentSocket
  (return (Variables|Sockets|GetAttachmentSocket)))

(fn SimulatePhysics
  (bind _component (CallFunction|GetPrimaryComponent))
  (Collision|SetCollisionProfileName _component "Ragdoll" true :!class /Script/Engine.PrimitiveComponent)
  (Physics|SetSimulatePhysics _component true))