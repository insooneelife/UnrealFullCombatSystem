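; DI_HandBP is a displayed-item Blueprint for equipment that moves between a regular attachment socket and a hand socket depending on combat state.
; Its GetAttachmentSocket returns the hand socket only when the owner is in combat and the slot is not hidden.
; It listens to the EquipmentComponent's slot-hidden event and re-attaches when its own slot changes during combat.
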(event Custom|OnSlotHiddenChanged
  (params (SlotType :type E_ItemType%20Enum :default "NewEnumerator0") (SlotIndex :type Integer) (ActiveItem :type F%20Stored%20Item%20Structure) (IsHidden :type Boolean))
  ;[1 0 0] Update attachment when item is hidden/unhidden
  (if (Default|GetIsinCombat (Variables|Default|GetEquipmentComponent))
    (if (and (Utilities|Enum|Equal(Enum) SlotType (Variables|Default|GetType)) (== (Variables|Default|GetSlotIndex) SlotIndex))
      (CallFunction|Attach))))

(event EventBeginPlay
  (|CallParentFunction)
  (EventDispatchers|AssignOnSlotHiddenChanged (Variables|Default|GetEquipmentComponent) (delegate Custom|OnSlotHiddenChanged)))

(fn ConstructionScript
  (|CallParentFunction))

(fn GetAttachmentSocket
  (if (Default|IsSlotHidden (Variables|Default|GetEquipmentComponent) (Variables|Default|GetType) (Variables|Default|GetSlotIndex))
    (return (Variables|Default|GetAttachmentSocket))
    (elif (Default|GetIsinCombat (Variables|Default|GetEquipmentComponent))
      (return (Variables|Sockets|GetHandAttachmentSocket))
      (else
        (return (Variables|Default|GetAttachmentSocket))))))