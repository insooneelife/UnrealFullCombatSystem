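; Usable potion item that modifies one of the user's stats, such as a restorative, by a configured amount.
; On use, it searches the caller's ExtendedStatComponentBP components for those matching its Type and applies Value without interrupting regeneration.
; Getters expose the displayed item and use montage, while the stat type and amount are variables, so the logic is not tied to a specific stat.
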(event EventUseItem
  (params (Caller :type Actor%20Object%20Reference))
  (for _array_element (Actor|GetComponentsByClass Caller "/Game/DynamicCombatSystem/Blueprints/Components/ExtendedStatComponentBP.ExtendedStatComponentBP_C")
    (if (Utilities|Enum|Equal(Enum) (Variables|/Game/DynamicCombatSystem/Blueprints/Components/ExtendedStatComponentBP.ExtendedStatComponentBP_C|GetType _array_element) (Variables|Potion|GetType))
      (Default|ModifyStat _array_element (Variables|Potion|GetValue) false))))

(fn GetDisplayedItem
  (return (Variables|Display|GetDisplayedItem)))

(fn GetUseMontage
  (return (Variables|Potion|GetUseMontage)))