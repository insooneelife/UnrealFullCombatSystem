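; Base character Blueprint for the Dynamic Combat System that drives camera zoom and blocking transitions.
; Condition-driven update events play or reverse two timelines: zoom sets an alpha and lerps the camera boom's arm length, while blocking sets a block alpha.
; When the blocking timeline finishes, its direction decides whether stamina regeneration is reduced or restored.
; Tick writes the selected main-hand type and current state to a text render component.
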(event EventBeginPlay)

(event Collision|EventActorBeginOverlap
  (params (OtherActor :type Actor%20Object%20Reference)))

(event EventTick
  (params (DeltaSeconds :type Float%20%28single-precision%29))
  (Rendering|Components|TextRender|SetText (Variables|Default|GetTextRender) (Utilities|Text|ToText(String) (Utilities|String|Append (Utilities|String|EnumtoString (Class|BaseCharacter|GetSelectedMainHandType)) "   " (Utilities|String|EnumtoString (Class|BaseCharacter|GetState)) "   "))))

(event EventUpdateZoomTimeline
  (params (bInCondition :type Boolean))
  (if bInCondition
    (bind _alpha (Timeline|ZoomingTimeline Play)
      (:Update
        (Class|BaseCharacter|SetZoomAlpha _alpha)
        (Variables|/Script/Engine.SpringArmComponent|SetTargetArmLength (Class|BaseCharacter|GetCameraBoom) (Math|Float|Lerp (Class|BaseCharacter|GetInitialCameraArmLength) (Class|BaseCharacter|GetZoomCameraArmLength) _alpha))))
    (else
      (Timeline|ZoomingTimeline Reverse))))

(event EventUpdateBlockingTimeline
  (params (bInCondition :type Boolean))
  (bind _returnvalue (Class|BaseCharacter|GetExtendedStaminaComp))
  (if bInCondition
    (bind (_direction _alpha) (Timeline|BlockingTimeline Play)
      (:Update
        (Class|BaseCharacter|SetBlockAlpha _alpha))
      (:Finished
        (switch Utilities|FlowControl|Switch|SwitchonETimelineDirection _direction
          (:Forward
            (Class|ExtendedStatComponent|ChangeRegenPercent _returnvalue 25))
          (:Backward
            (Class|ExtendedStatComponent|ChangeRegenPercent _returnvalue 100)))))
    (else
      (Timeline|BlockingTimeline Reverse))))

(fn ConstructionScript)