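; AI ability that instantly heals the owning character by a set amount.
; On release it asks the ability component to start, then plays its montage scaled by casting speed.
; The effect event raises the owner's Health stat without interrupting regeneration, plays an attached sound, spawns a heal particle on the character mesh and consumes mana.
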(event Custom|SpawnParticle
  ;[0 0.272 1] Spawn heal particle
  (Effects|SpawnEmitterAttached (Variables|Default|GetHealParticle) (Variables|/Script/Engine.Character|GetMesh (Class|AbilityBase|GetCharacter)) "" "0, 0,20.000000"))

(event Custom|PlaySound
  ;[0 0.272 1] Play Sound
  (Audio|SpawnSoundAttached (Variables|Default|GetSound) (Variables|/Script/Engine.Character|GetMesh (Class|AbilityBase|GetCharacter)) "None" "0, 0, 0" "0, 0, 0" "KeepRelativeOffset" false 1.0 1.0 0.0 0 0))

(event EventEffect
  ;[0 0.272 1] On effect heal owner
  (CallFunction|Heal)
  (CallFunction|PlaySound)
  (CallFunction|SpawnParticle)
  (Class|AbilityBase|ConsumeMana))

(event EventReleased
  ;[0 0.272 1] On released check whether ability can be started and play montage
  (bind _returnvalue (Class|AbilityComponent|StartAbility (Class|AbilityBase|GetAbilityComponent)))
  (if _returnvalue
    (Class|AbilityBase|PlayAbilityMontage (Class|AbilityBase|GetAbilityMontage) "None" true 1.0)))

(fn ConstructionScript)

(fn Heal
  (Class|ExtendedStatComponent|ModifyStat (Class|DefaultGameInstance|GetExtendedStatComponent (Class|AIAbilityBase|GetAICharacter) "Health") (Variables|Default|GetHealAmount) false))