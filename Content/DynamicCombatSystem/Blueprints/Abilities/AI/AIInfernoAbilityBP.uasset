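; AI ability Blueprint for Inferno, an area damage attack cast at a predicted target position on a surface.
; On Released, it starts the ability, plays the montage at casting speed, fixes the effect transform within range and shows an indicator there.
; The Effect event spawns and initializes a damage sphere actor with radius, damage and impulse, plays the particle and sound, then consumes mana.
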(event Custom|SpawnParticle
  ;[0 0.272 1] Spawn Particle
  (Effects|SpawnEmitteratLocation (Variables|Default|GetHitParticle) (Class|AbilityBase|GetEffectLocation)))

(event Custom|PlaySound
  ;[0 0.272 1] Play Sound
  (Audio|PlaySoundatLocation (Variables|Default|GetSound) (Class|AbilityBase|GetEffectLocation) "0, 0, 0" 1.0 1.0 0.0 0 0 0))

(event EventEffect
  (bind _returnvalue (Components|GetOwner))
  ;[0 0.272 1] On effect spawn damage sphere
  (bind _returnvalue_2 (Game|SpawnActorfromClass "/Game/DynamicCombatSystem/Blueprints/AbilityEffects/DamageSphereEffectBP.DamageSphereEffectBP_C" (Class|AbilityBase|GetEffectTransform) "AlwaysSpawn" _returnvalue (Game|GetInstigator _returnvalue)))
  (Class|DamageSphereAbilityEffect|Init _returnvalue_2 (Variables|Default|GetRadius) (Class|AbilityBase|GetDamage) (Class|AbilityBase|GetImpulsePower))
  (CallFunction|SpawnParticle)
  (CallFunction|PlaySound)
  (Class|AbilityBase|ConsumeMana))

(event EventReleased
  ;[0 0.272 1] On Pressed play anim montage, update effect transform and show indicator
  (bind _returnvalue (Class|AbilityComponent|StartAbility (Class|AbilityBase|GetAbilityComponent)))
  (if _returnvalue
    (Class|AbilityBase|PlayAbilityMontage (Class|AbilityBase|GetAbilityMontage) "None" true 1.0)
    (Class|AbilityBase|SetEffectTransform (Class|AIAbilityBase|GetSurfacePredictedTargetTransform (Variables|Default|GetRange)))
    (Class|AbilityBase|ShowIndicator (Class|AbilityBase|GetEffectLocation))))

(fn ConstructionScript)