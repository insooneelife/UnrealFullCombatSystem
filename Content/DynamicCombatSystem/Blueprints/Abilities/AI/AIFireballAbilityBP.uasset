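; AI fireball ability that spawns a fireball projectile aimed at the target and consumes mana.
; Release plays a cast montage, using the first initially, then cycling the rest until a retriggerable delay resets it, with the hand socket matched per montage.
; A looping timer, instead of Tick, handles effect aiming until the cast fires or ends.
; The projectile's Init call for damage and homing target is not wired to execution.
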(event Custom|ResetMontageCounter
  ;[0 0.272 1] When casted first, use montage at index 0 and then if keeps casting, use montages at indexes 1 & 2
  (Variables|Default|SetMontageCounter 0))

(event Custom|UpdateMontageCounter
  ;[0 0.272 1] When casted first, use montage at index 0 and then if keeps casting, use montages at indexes 1 & 2
  (bind _result (Math|Integer|IncrementInt (Variables|Default|GetMontageCounter))
    (:%20%20
      (if (> _result (Utilities|Array|LastIndex (Class|AbilityBase|GetAbilityMontages)))
        (Variables|Default|SetMontageCounter 1)))))

(event Custom|UpdateSocket
  ;[0 0.272 1] Use left hand socket only for 1st index because animation at this index uses left hand
  (switch int (Variables|Default|GetMontageCounter)
    (:0
      (Variables|Default|SetUseLeftHandSocket false))
    (:1
      (Variables|Default|SetUseLeftHandSocket true))
    (:2
      (Variables|Default|SetUseLeftHandSocket false))))

(event Custom|UpdateEffect
  (bind _returnvalue (Class|AbilityBase|GetCharacter))
  (bind _returnvalue_2 (Class|AbilityBase|GetRightHandSocket))
  (bind _returnvalue_3 (Class|AbilityBase|GetLeftHandSocket))
  (bind _returnvalue_4 (Class|AIAbilityBase|GetTargetLoc))
  (bind _uselefthandsocket (Variables|Default|GetUseLeftHandSocket))
  (bind _returnvalue_5 (select _uselefthandsocket _returnvalue_3 _returnvalue_2))
  (bind _mesh (Variables|/Script/Engine.Character|GetMesh _returnvalue))
  (bind _returnvalue_6 (Transformation|GetSocketLocation _mesh _returnvalue_5))
  (bind _returnvalue_7 (Math|Rotator|FindLookatRotation _returnvalue_6 _returnvalue_4))
  ;[0 0.272 1] Update effect transform
  (Class|AbilityBase|SetEffectTransform (Math|Transform|MakeTransform (+ _returnvalue_6 (Math|Rotator|GetRotationXVector _returnvalue_7)) _returnvalue_7)))

(event Custom|StartTimer
  ;[0 0.272 1] Use timer updating ability effect instead of doing it on tick
  (Utilities|Time|SetTimerbyEvent (EventDispatchers|CreateEvent :!event Custom|UpdateEffect) 0.016 true))

(event Custom|StopTimer
  ;[0 0.272 1] Use timer updating ability effect instead of doing it on tick
  (Utilities|Time|ClearTimerbyFunctionName 0 "UpdateEffect"))

(event EventReleased
  ;[0 0.272 1] On released check whether ability can be started and update montage index and play it
  (bind _returnvalue (Class|AbilityComponent|StartAbility (Class|AbilityBase|GetAbilityComponent)))
  (if _returnvalue
    (CallFunction|StartTimer)
    (CallFunction|UpdateSocket)
    (bind _returnvalue_2 (Class|AbilityBase|PlayAbilityMontage (Class|AbilityBase|GetAbilityMontage (Variables|Default|GetMontageCounter)) "None" true 1.0))
    (CallFunction|UpdateMontageCounter)
    (Utilities|FlowControl|RetriggerableDelay _returnvalue_2)
    (CallFunction|ResetMontageCounter)))

(event EventEffect
  (bind _returnvalue (Components|GetOwner))
  (bind _returnvalue_2 (Game|GetInstigator _returnvalue))
  ;[0 0.272 1] On effect spawn homing projectile
  (CallFunction|UpdateEffect)
  (bind _returnvalue_3 (Game|SpawnActorfromClass "/Game/DynamicCombatSystem/Blueprints/AbilityEffects/FireballProjectileEffectBP.FireballProjectileEffectBP_C" (Class|AbilityBase|GetEffectTransform) "AlwaysSpawn" _returnvalue_2 _returnvalue_2))
  (CallFunction|StopTimer)
  (Class|AbilityBase|ConsumeMana))

(event EventEnded
  (params (Result :type EAbilityEndResult%20Enum :default "Finished"))
  ;[0 0.272 1] Stop timer updating effect when ability ends
  (CallFunction|StopTimer))

(fn ConstructionScript)