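; AI ability that summons a minion near the caster to fight the caster's current target.
; On release it runs an EQS query for a summon spot, snaps the result to the ground and plays the casting montage, or ends as interrupted if no valid spot is found.
; The Effect event spawns the minion facing the target, sets its owner and AI target, plays a sound and consumes mana.
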(event Custom|OnQueryFinishedEvent
  (params (QueryInstance :type Env%20Query%20Instance%20Blueprint%20Wrapper%20Object%20Reference) (QueryStatus :type EEnvQueryStatus%20Enum :default "Processing"))
  ;[0 0.272 1] When EQS query finish, save teleport location in EffectTransform variable and play anim montage
  (bind (_resultlocations _returnvalue) (AI|EQS|GetQueryResultsasLocations QueryInstance))
  (if _returnvalue
    (if (.ReturnValue (Class|AbilityBase|FindGroundLocation (Utilities|Array|Get(acopy) _resultlocations) 8e+01))
      (Class|AbilityBase|SetEffectTransform (Math|Transform|MakeTransform (.OutGroundLocation (Class|AbilityBase|FindGroundLocation (Utilities|Array|Get(acopy) _resultlocations) 8e+01)) (Math|Conversions|RotationFromXVector (Math|Vector|GetUnitDirection(Vector) (Transformation|GetActorLocation (Components|GetOwner)) (.OutGroundLocation (Class|AbilityBase|FindGroundLocation (Utilities|Array|Get(acopy) _resultlocations) 8e+01))))))
      (Class|AbilityBase|PlayAbilityMontage (Class|AbilityBase|GetAbilityMontage) "None" true 1.0)
      (else
        (Class|AbilityComponent|EndAbility (Class|AbilityBase|GetAbilityComponent) "Interrupted" :!label _label)))
    (else
      (goto _label))))

(event Custom|PlaySound
  ;[0 0.272 1] Play Sound
  (Audio|PlaySoundatLocation (Variables|Default|GetSound) (Class|AbilityBase|GetEffectLocation) "0, 0, 0" 1.0 1.0 0.0 0 0 0))

(event EventEffect
  ;[0 0.272 1] On ability effect teleport character
  (CallFunction|SummonMinion)
  (CallFunction|PlaySound)
  (Class|AbilityBase|ConsumeMana))

(event EventReleased
  ;[0 0.272 1] On Pressed check whether ability can be started
  (bind _returnvalue (Class|AbilityComponent|StartAbility (Class|AbilityBase|GetAbilityComponent)))
  (if _returnvalue
    ;[0 0.272 1] Run EQS Query to find teleport location
    (bind _returnvalue_2 (AI|EQS|RunEQSQuery "/Game/DynamicCombatSystem/Blueprints/AI/EQS/EQS_SummonSpot2.EQS_SummonSpot2" (Components|GetOwner) "RandomBest25Pct"))
    (EventDispatchers|AssignOnQueryFinishedEvent _returnvalue_2 (EventDispatchers|CreateEvent :!event Custom|OnQueryFinishedEvent))))

(fn ConstructionScript)

(fn SummonMinion
  (bind _returnvalue (AI|SpawnAIFromClass (Variables|Default|GetSpawnedMinion) 0 (Class|AbilityBase|GetEffectLocation) (Math|Rotator|MakeRotator 0.0 0.0 (.Yaw (Math|Rotator|BreakRotator (Math|Rotator|FindLookatRotation (Class|AbilityBase|GetEffectLocation) (Class|AIAbilityBase|GetTargetLoc))))) true 0))
  (Actor|SetOwner _returnvalue (Components|GetOwner))
  (bind _asaicharacter (Utilities|Casting|CastToAICharacter _returnvalue))
  (Class|BaseAIController|SetTarget (Class|AICharacter|GetAIController _asaicharacter) (Class|AIAbilityBase|GetTarget)))