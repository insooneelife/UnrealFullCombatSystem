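; AI trap ability for the Dynamic Combat System that places a timed damage trap on a targeted surface within range.
; On release it starts the ability, plays the cast montage, stores the surface target transform and shows an indicator there.
; The Effect event spawns and initializes a DamageTrapEffectBP at that stored transform, passing damage, impulse, radii, duration and activation delay, then plays a sound and consumes mana.
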(event Custom|PlaySound
  ;[0 0.272 1] Play Sound
  (Audio|PlaySoundatLocation (Variables|Default|GetSound) (Class|AbilityBase|GetEffectLocation) "0, 0, 0" 1.0 1.0 0.0 0 0 0))

(event EventEffect
  (bind _returnvalue (Components|GetOwner))
  ;[0 0.272 1] On ability effect spawn trap
  (bind _returnvalue_2 (Game|SpawnActorfromClass "/Game/DynamicCombatSystem/Blueprints/AbilityEffects/DamageTrapEffectBP.DamageTrapEffectBP_C" (Class|AbilityBase|GetEffectTransform) "AlwaysSpawn" _returnvalue (Game|GetInstigator _returnvalue)))
  (Class|DamageTrapAbilityEffect|Init _returnvalue_2 (Variables|Default|GetDamageRadius) (Class|AbilityBase|GetDamage) (Class|AbilityBase|GetImpulsePower) (Variables|Default|GetTrapRadius) (Variables|Default|GetDuration) (Variables|Default|GetActivationDelay))
  (CallFunction|PlaySound)
  (Class|AbilityBase|ConsumeMana))

(event EventReleased
  ;[0 0.272 1] On Pressed play anim montage, update effect transform and show indicator
  (bind _returnvalue (Class|AbilityComponent|StartAbility (Class|AbilityBase|GetAbilityComponent)))
  (if _returnvalue
    (Class|AbilityBase|PlayAbilityMontage (Class|AbilityBase|GetAbilityMontage) "None" true 1.0)
    (Class|AbilityBase|SetEffectTransform (Class|AIAbilityBase|GetSurfaceTargetTransform (Variables|Default|GetRange)))
    (Class|AbilityBase|ShowIndicator (Class|AbilityBase|GetEffectLocation))))

(fn ConstructionScript)

(fn SpawnTrap)