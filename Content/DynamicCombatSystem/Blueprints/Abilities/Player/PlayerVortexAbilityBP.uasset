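; Channeled player vortex ability that drains mana while damaging and pushing pawns it touches.
; Pressed shows an indicator and retries casting on a timer until it succeeds; Released or running out of mana plays the montage's End section.
; While active, Tick glides particle and sound toward the surface-traced target at constant speed.
; A capsule trace at the particle hits each actor once per check, applying damage and impulse.
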(event Custom|SpawnParticle
  ;[0 0.272 1] Vortex Particle
  (bind _particlecomponent (Variables|Default|GetParticleComponent)
    (:then
      (Components|Activation|Activate _particlecomponent false)
      (Transformation|SetWorldLocation _particlecomponent (Variables|NonEdit|GetVortexLocation) false false))
    (:else
      (bind _returnvalue (Effects|SpawnEmitteratLocation (Variables|Ability|Custom|GetVortexParticle) (Variables|NonEdit|GetVortexLocation)))
      (Variables|Default|SetParticleComponent _returnvalue))))

(event Custom|DeactivateParticle
  ;[0 0.272 1] Vortex Particle
  (bind _particlecomponent (Variables|Default|GetParticleComponent)
    (:then
      (Components|Activation|Deactivate _particlecomponent))
    (:else)))

(event Custom|PlaySound
  ;[0 0.272 1] Sound
  (bind _soundcomponent (Variables|Default|GetSoundComponent)
    (:then
      (Transformation|SetWorldLocation _soundcomponent (Variables|NonEdit|GetVortexLocation) false false))
    (:else
      (bind _returnvalue (Audio|SpawnSoundatLocation (Variables|Ability|Custom|GetSound) (Variables|NonEdit|GetVortexLocation) "0, 0, 0" 1.0 1.0 0.0 0 0))
      (Variables|Default|SetSoundComponent _returnvalue)))
  (Audio|Components|Audio|FadeIn (Variables|Default|GetSoundComponent) 0.5 1.0 0.0 "Linear" :!class /Script/Engine.AudioComponent))

(event Custom|AttempToCastEvent
  ;[0 0.272 1] On Pressed attempt to cast ability until it succeed or gets interrupted
  (CallFunction|AttempttoCast))

(event Custom|ClearAttemptToCastTimer
  ;[0 0.272 1] Clear Attempt To Cast Timer
  (Utilities|Time|ClearTimerbyFunctionName 0 "AttempToCastEvent"))

(event Custom|StopSound
  ;[0 0.272 1] Sound
  (bind _soundcomponent (Variables|Default|GetSoundComponent)
    (:then
      (Audio|Components|Audio|FadeOut _soundcomponent 0.5 0.0 "Linear" :!class /Script/Engine.AudioComponent))
    (:else)))

(event Custom|UpdateVortex
  ;[0 0.272 1] Update vortex location, then location of particle & sound
  (Variables|NonEdit|SetVortexLocation (Math|Interpolation|VInterptoConstant (Variables|NonEdit|GetVortexLocation) (Class|AbilityBase|GetEffectLocation) (Utilities|Time|GetWorldDeltaSeconds) (Variables|Ability|Custom|GetVortexSpeed)))
  (Utilities|FlowControl|Sequence
    (:then_0
      (bind _particlecomponent (Variables|Default|GetParticleComponent)
        (:then
          (Transformation|SetWorldLocationAndRotation _particlecomponent (Variables|NonEdit|GetVortexLocation) "0, 0, 0" false false))
        (:else)))
    (:then_1
      (bind _soundcomponent (Variables|Default|GetSoundComponent)
        (:then
          (Transformation|SetWorldLocation _soundcomponent (Variables|NonEdit|GetVortexLocation) false false))
        (:else)))))

(event EventPressed
  ;[0 0.272 1] On Pressed attempt to cast ability until it succeed or gets interrupted
  (Class|AbilityBase|ShowIndicator (Class|AbilityBase|GetEffectLocation))
  (bind _result (CallFunction|AttempttoCast))
  (if (not _result)
    (Utilities|Time|SetTimerbyEvent (delegate Custom|AttempToCastEvent) 0.1 true)))

(event EventEnded
  (params (Result :type EAbilityEndResult%20Enum :default "Finished"))
  ;[0 0.272 1] End of ability events
  (CallFunction|ClearAttempttoCastTimer)
  (Variables|NonEdit|SetEffectEnabled false)
  (CallFunction|DeactivateParticle)
  (CallFunction|StopSound)
  (switch Utilities|FlowControl|Switch|SwitchonEAbilityEndResult Result
    (:OutOfMana
      (Class|AbilityBase|PlayAbilityMontage (Class|AbilityBase|GetAbilityMontage) "End" true 1.0))))

(event EventReleased
  ;[0 0.272 1] On released stop ability
  (CallFunction|ClearAttempttoCastTimer)
  (if (Class|AbilityComponent|IsCasting (Class|AbilityBase|GetAbilityComponent))
    (Class|AbilityBase|PlayAbilityMontage (Class|AbilityBase|GetAbilityMontage) "End" true 1.0)
    (Class|AbilityComponent|EndAbility (Class|AbilityBase|GetAbilityComponent) "Finished")))

(event EventTick
  (params (DeltaSeconds :type Float%20%28single-precision%29))
  ;[0 0.272 1] Tick, update effect transform, spell indicator, check for enemies and cosume mana
  (Utilities|FlowControl|Sequence
    (:then_0
      (if (Class|AbilityComponent|IsUsingAbility (Class|AbilityBase|GetAbilityComponent))
        (Class|AbilityBase|SetEffectTransform (Class|PlayerAbilityBase|GetSurfaceTransform (Variables|Ability|Custom|GetRange) (Variables|Ability|Custom|GetMaxSurfaceAngle) 2e+03))
        (Class|AbilityComponent|UpdateSpellIndicatorLocation (Class|AbilityBase|GetAbilityComponent) (Class|AbilityBase|GetEffectLocation))))
    (:then_1
      (if (Variables|NonEdit|GetEffectEnabled)
        (CallFunction|UpdateVortex)
        (CallFunction|CheckforEnemies)
        (Class|AbilityBase|ConsumeMana)))))

(event EventEffect
  ;[0 0.272 1] Effect
  (Variables|NonEdit|SetEffectEnabled true)
  (Variables|NonEdit|SetVortexLocation (Class|AbilityBase|GetEffectLocation))
  (CallFunction|PlaySound)
  (CallFunction|SpawnParticle)
  (Class|AbilityBase|ConsumeManaAmount (Variables|Ability|Custom|GetFirstUseManaCost)))

(fn ConstructionScript
  (|CallParentFunction))

(fn CheckforEnemies
  (bind _returnvalue (Components|GetOwner))
  (bind _collisionheight (Variables|Ability|Custom|GetCollisionHeight))
  (bind _particlecomponent (Variables|Default|GetParticleComponent))
  (bind _returnvalue_2 (Transformation|GetWorldLocation _particlecomponent))
  (bind (_x _y _z) (Math|Vector|BreakVector _returnvalue_2))
  (bind _returnvalue_3 (+ _z _collisionheight))
  (bind _returnvalue_4 (Math|Vector|MakeVector _x _y _returnvalue_3))
  (bind _outhits (Class|KismetSystemLibrary|CapsuleTraceMultiforObjects _returnvalue_4 (+ _returnvalue_4 "0, 0,1.000000") (Variables|Ability|Custom|GetRadius) (Variables|Ability|Custom|GetCollisionHeight) (Utilities|Array|MakeArray "ObjectTypeQuery3") false (Utilities|Array|MakeArray (Components|GetOwner)) "None" true))
  (for _array_element _outhits
    (if (not (Utilities|Array|ContainsItem (LocalVariables|GetL_HitActors) (.HitActor (Collision|BreakHitResult _array_element))))
      (Utilities|Array|Add (LocalVariables|GetL_HitActors) (.HitActor (Collision|BreakHitResult _array_element)))
      (bind _ascan_be_attacked (Utilities|Casting|CastToCanBeAttacked (.HitActor (Collision|BreakHitResult _array_element))))
      (Class|CanbeAttacked|TakeDamage _ascan_be_attacked (Utilities|Struct|MakeHitData (Class|AbilityBase|GetDamage) _returnvalue (Math|Vector|GetUnitDirection(Vector) (Transformation|GetActorLocation _returnvalue) (Transformation|GetActorLocation (.HitActor (Collision|BreakHitResult _array_element)))) false true false))
      (Class|AbilityBase|ApplyImpulsetoCharacter (.HitActor (Collision|BreakHitResult _array_element)) (.Normal (Collision|BreakHitResult _array_element)) (Class|AbilityBase|GetImpulsePower)))))

(fn AttempttoCast
  (bind _returnvalue (Class|AbilityComponent|StartAbility (Class|AbilityBase|GetAbilityComponent)))
  (if _returnvalue
    (Class|AbilityBase|PlayAbilityMontage (Class|AbilityBase|GetAbilityMontage) "None" true 1.0)
    (CallFunction|ClearAttempttoCastTimer)
    (return true)
    (else
      (return false))))