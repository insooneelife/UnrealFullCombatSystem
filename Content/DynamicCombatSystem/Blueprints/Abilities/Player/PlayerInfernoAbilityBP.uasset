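; Player inferno ability that deals area damage at an aimed surface location within range.
; While the input is held and not casting, Tick moves the effect transform and indicator via GetSurfaceTransform, limited by surface angle.
; Release starts the ability and montage, or hides the indicator if it cannot start and is not casting.
; Effect spawns a damage sphere and particle there, consumes mana and plays a sound.
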(event Custom|SpawnParticle
  ;[0 0.272 1] Spawn Particle
  (Effects|SpawnEmitteratLocation (Variables|Ability|Custom|GetHitParticle) (Class|AbilityBase|GetEffectLocation)))

(event Custom|UpdateEffect
  ;[0 0.272 1] Update effect transform and it's indicator
  (Class|AbilityBase|SetEffectTransform (Class|PlayerAbilityBase|GetSurfaceTransform (Variables|Ability|Custom|GetRange) (Variables|Ability|Custom|GetMaxSurfaceAngle) 0.0))
  (Class|AbilityBase|UpdateIndicator (Class|AbilityBase|GetEffectLocation)))

(event Custom|PlaySound
  ;[0 0.272 1] Play Sound
  (Audio|PlaySoundatLocation (Variables|Ability|Custom|GetSound) (Class|AbilityBase|GetEffectLocation) "0, 0, 0" 1.0 1.0 0.0 0 0 0))

(event Custom|Pressed_1
  ;[0 0.272 1] On Ability pressed show spell indicator if not casting
  (if (not (Class|AbilityComponent|GetIsCasting (Class|AbilityBase|GetAbilityComponent)))
    (CallFunction|UpdateEffect)
    (Class|AbilityBase|ShowIndicator (Class|AbilityBase|GetEffectLocation))))

(event EventReleased
  (bind _returnvalue (Class|AbilityBase|GetAbilityComponent))
  ;[0 0.272 1] On Ability released cast ability or hide spell indicator if not casting
  (bind _returnvalue_2 (Class|AbilityComponent|StartAbility _returnvalue))
  (if _returnvalue_2
    (Class|AbilityBase|PlayAbilityMontage (Class|AbilityBase|GetAbilityMontage) "None" false 0.0)
    (CallFunction|UpdateEffect)
    (elif (not (Class|AbilityComponent|GetIsCasting _returnvalue))
      (Class|AbilityBase|HideIndicator))))

(event EventTick
  (params (DeltaSeconds :type Float%20%28single-precision%29))
  (bind _returnvalue (Class|AbilityBase|GetAbilityComponent))
  ;[0 0.272 1] Update effect transform only if ability is pressed but not already casting
  (if (and (Class|AbilityComponent|GetIsPressed _returnvalue) (not (Class|AbilityComponent|GetIsCasting _returnvalue)))
    (CallFunction|UpdateEffect)))

(event EventEffect
  (bind _returnvalue (Components|GetOwner))
  ;[0 0.272 1] Effect
  (Game|SpawnActorfromClass "/Game/DynamicCombatSystem/Blueprints/AbilityEffects/AE_DamageSphere.AE_DamageSphere_C" (Class|AbilityBase|GetEffectTransform) "AlwaysSpawn" _returnvalue (Variables|Ability|Custom|GetRadius) (Class|AbilityBase|GetDamage) (Class|AbilityBase|GetImpulsePower) "None" (Game|GetInstigator _returnvalue))
  (CallFunction|SpawnParticle)
  (Class|AbilityBase|ConsumeMana)
  (CallFunction|PlaySound))

(fn ConstructionScript
  (|CallParentFunction))

(fn UpdateEffectTransform
  (bind _returnvalue (Class|AbilityBase|GetEffectLocation))
  (bind _returnvalue_2 (Components|GetOwner))
  (bind _returnvalue_3 (Transformation|GetActorLocation _returnvalue_2))
  (bind _z (Math|Vector|BreakVector _returnvalue))
  ;[0 0.272 1] Calculate Start/End trace location
  (LocalVariables|SetL_TraceStart _returnvalue_3)
  (LocalVariables|SetL_TraceEnd (+ _returnvalue_3 (* (Transformation|GetActorForwardVector (Pawn|GetController (Variables|/Script/Engine.Actor|GetInstigator _returnvalue_2))) (Variables|Ability|Custom|GetRange))))
  (bind _outhit (Collision|LineTraceForObjects (LocalVariables|GetL_TraceStart) (LocalVariables|GetL_TraceEnd) (Utilities|Array|MakeArray "ObjectTypeQuery1") false 0 "None"))
  (if (.bBlockingHit (Collision|BreakHitResult _outhit))
    (LocalVariables|SetL_HitLocation (.Location (Collision|BreakHitResult _outhit)))
    (if (<= (Class|KismetMathLibrary|DegAcos (Math|Vector|DotProduct (.Normal (Collision|BreakHitResult _outhit)) "0, 0,1.000000")) (Math|Float|Absolute(Float) (Variables|Ability|Custom|GetMaxSurfaceAngle)))
      (LocalVariables|SetL_EffectLocation (LocalVariables|GetL_HitLocation))
      (else
        (LocalVariables|SetL_EffectLocation (Math|Vector|MakeVector (.X (Math|Vector|BreakVector (LocalVariables|GetL_HitLocation))) (.Y (Math|Vector|BreakVector (LocalVariables|GetL_HitLocation))) _z))))
    (else
      (LocalVariables|SetL_EffectLocation (Math|Vector|MakeVector (.X (Math|Vector|BreakVector (LocalVariables|GetL_TraceEnd))) (.Y (Math|Vector|BreakVector (LocalVariables|GetL_TraceEnd))) _z))))
  (return (Math|Transform|MakeTransform (LocalVariables|GetL_EffectLocation))))