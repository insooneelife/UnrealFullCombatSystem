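; Player fireball ability in the Dynamic Combat System that fires a stunning projectile along the crosshair transform and consumes mana.
; On release it starts the ability and plays a casting montage, opening with the first and alternating between the next two on continued casts.
; A retriggerable delay based on montage playback resets that chain when casting stops.
; The Effect event spawns and initializes the projectile from the hand socket matched to the current animation.
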(event Custom|ResetMontageCounter
  ;[0 0.272 1] When casted first, use montage at index 0 and then if keeps casting, use montages at indexes 1 & 2
  (Variables|NonEdit|SetMontageCounter 0))

(event Custom|UpdateMontageCounter
  ;[0 0.272 1] When casted first, use montage at index 0 and then if keeps casting, use montages at indexes 1 & 2
  (bind _result (Math|Integer|IncrementInt (Variables|NonEdit|GetMontageCounter))
    (:%20%20
      (if (> _result (Utilities|Array|LastIndex (Class|AbilityBase|GetAbilityMontages)))
        (Variables|NonEdit|SetMontageCounter 1)))))

(event Custom|UpdateSocket
  ;[0 0.272 1] Use left hand socket only for 1st index because animation at this index uses left hand
  (switch int (Variables|NonEdit|GetMontageCounter)
    (:0
      (Variables|NonEdit|SetUseLeftHandSocket false))
    (:1
      (Variables|NonEdit|SetUseLeftHandSocket true))
    (:2
      (Variables|NonEdit|SetUseLeftHandSocket false))))

(event EventReleased
  (bind _returnvalue (Class|AbilityComponent|StartAbility (Class|AbilityBase|GetAbilityComponent)))
  (if _returnvalue
    (CallFunction|UpdateSocket)
    (bind _returnvalue_2 (Class|AbilityBase|PlayAbilityMontage (Class|AbilityBase|GetAbilityMontage (Variables|NonEdit|GetMontageCounter)) "None" true 1.0))
    ;[0 0.272 1] Handle montage counter
    (CallFunction|UpdateMontageCounter)
    (Utilities|FlowControl|RetriggerableDelay _returnvalue_2)
    (CallFunction|ResetMontageCounter)))

(event EventEffect
  (bind _returnvalue (Class|AbilityBase|GetRightHandSocket))
  (bind _returnvalue_2 (Class|AbilityBase|GetLeftHandSocket))
  (bind _returnvalue_3 (Components|GetOwner))
  (bind _uselefthandsocket (Variables|NonEdit|GetUseLeftHandSocket))
  (bind _returnvalue_4 (select _uselefthandsocket _returnvalue_2 _returnvalue))
  (bind _returnvalue_5 (Class|PlayerAbilityBase|GetCrosshairTransform _returnvalue_4))
  ;[0 0.272 1] Spawn Fireball projectile and consume mana
  (Class|AbilityBase|SetEffectTransform _returnvalue_5)
  (bind _returnvalue_6 (Game|SpawnActorfromClass "/Game/DynamicCombatSystem/Blueprints/AbilityEffects/FireballProjectileEffectBP.FireballProjectileEffectBP_C" _returnvalue_5 "AdjustIfPossibleButAlwaysSpawn" _returnvalue_3 (Game|GetInstigator _returnvalue_3)))
  (Class|FireballProjectileAbilityEffect|Init _returnvalue_6 (Class|AbilityBase|GetDamage) (Variables|Ability|Custom|GetInitialProjectileSpeed) 1e+01 0 true)
  (Class|AbilityBase|ConsumeMana))

(fn ConstructionScript
  (|CallParentFunction))