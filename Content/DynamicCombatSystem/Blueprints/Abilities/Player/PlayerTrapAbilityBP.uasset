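; Player ability in the Dynamic Combat System that places a damage trap on a surface.
; While pressed and not casting, it updates a ground indicator from a surface transform limited by range, angle and height deviation.
; Releasing starts the ability and plays the cast montage, or hides the indicator if it cannot start and is not casting.
; The Effect event spawns and initializes the trap actor at that transform, consumes mana and plays a sound.
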(event Custom|PlaySound
  ;[0 0.272 1] Play Sound
  (Audio|PlaySoundatLocation (Variables|Ability|Custom|GetSound) (Class|AbilityBase|GetEffectLocation) "0, 0, 0" 1.0 1.0 0.0 0 0 0))

(event Custom|UpdateEffect
  ;[0 0.272 1] Update effect transform and it's indicator
  (Class|AbilityBase|SetEffectTransform (Class|PlayerAbilityBase|GetSurfaceTransform (Variables|Ability|Custom|GetRange) (Variables|Ability|Custom|GetMaxSurfaceAngle) (Variables|Ability|Custom|GetMaxHeightDeviation)))
  (Class|AbilityBase|UpdateIndicator (Class|AbilityBase|GetEffectLocation)))

(event EventTick
  (params (DeltaSeconds :type Float%20%28single-precision%29))
  (bind _returnvalue (Class|AbilityBase|GetAbilityComponent))
  ;[0 0.272 1] Update effect transform only if ability is pressed but not already casting
  (if (and (Class|AbilityComponent|GetIsPressed _returnvalue) (not (Class|AbilityComponent|GetIsCasting _returnvalue)))
    (CallFunction|UpdateEffect)))

(event EventReleased
  ;[0 0.272 1] On Ability released cast ability or hide spell indicator if not casting
  (bind _returnvalue (Class|AbilityComponent|StartAbility (Class|AbilityBase|GetAbilityComponent)))
  (if _returnvalue
    (Class|AbilityBase|PlayAbilityMontage (Class|AbilityBase|GetAbilityMontage) "None" true 1.0)
    (CallFunction|UpdateEffect)
    (elif (not (Class|AbilityComponent|GetIsCasting (Class|AbilityBase|GetAbilityComponent)))
      (Class|AbilityBase|HideIndicator))))

(event EventPressed
  ;[0 0.272 1] On Ability pressed show spell indicator
  (if (not (Class|AbilityComponent|GetIsCasting (Class|AbilityBase|GetAbilityComponent)))
    (CallFunction|UpdateEffect)
    (Class|AbilityBase|ShowIndicator (Class|AbilityBase|GetEffectLocation))))

(event EventEffect
  (bind _returnvalue (Components|GetOwner))
  ;[0 0.272 1] Effect
  (bind _returnvalue_2 (Game|SpawnActorfromClass "/Game/DynamicCombatSystem/Blueprints/AbilityEffects/DamageTrapEffectBP.DamageTrapEffectBP_C" (Class|AbilityBase|GetEffectTransform) "AlwaysSpawn" _returnvalue (Game|GetInstigator _returnvalue)))
  (Class|DamageTrapAbilityEffect|Init _returnvalue_2 (Variables|Ability|Custom|GetDamageRadius) (Class|AbilityBase|GetDamage) (Class|AbilityBase|GetImpulsePower) (Variables|Ability|Custom|GetTrapRadius) (Variables|Ability|Custom|GetDuration) (Variables|Ability|Custom|GetActivationDelay))
  (Class|AbilityBase|ConsumeMana)
  (CallFunction|PlaySound))

(fn ConstructionScript
  (|CallParentFunction))