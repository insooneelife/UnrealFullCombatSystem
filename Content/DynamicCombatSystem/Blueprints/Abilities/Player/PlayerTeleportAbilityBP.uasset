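; Player teleport ability for the Dynamic Combat System that moves the owner to an aimed surface point.
; While held and not casting, it updates the target via GetSurfaceTransform and shows an indicator; release starts the ability and plays its montage.
; The Effect event teleports the owner, lifted by capsule half height, then consumes mana and plays particle and sound on success.
; A separate line-trace targeting function, UpdateEffectTransform, goes uncalled here.
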(event Custom|PlaySound
  ;[0 0.272 1] Play Sound
  (Audio|SpawnSoundAttached (Variables|Ability|Custom|GetSound) (Variables|/Script/Engine.Character|GetMesh (Class|AbilityBase|GetCharacter)) "None" "0, 0, 0" "0, 0, 0" "KeepRelativeOffset" false 1.0 1.0 0.0 0 0))

(event Custom|UpdateEffect
  ;[0 0.272 1] Update effect transform and it's indicator
  (Class|AbilityBase|SetEffectTransform (Class|PlayerAbilityBase|GetSurfaceTransform (Variables|Ability|Custom|GetRange) (Variables|Ability|Custom|GetMaxSurfaceAngle) 0.0))
  (Class|AbilityBase|UpdateIndicator (Class|AbilityBase|GetEffectLocation)))

(event Custom|SpawnTeleportParticle
  ;[0 0.272 1] Spawn Teleport Particle
  (Effects|SpawnEmitterAttached (Variables|Ability|Custom|GetTeleportParticle) (Variables|/Script/Engine.Character|GetMesh (Class|AbilityBase|GetCharacter)) "spine_01" "0, 0,-50.000000"))

(event EventEffect
  ;[0 0.272 1] Effect
  (bind _result (CallFunction|AbilityTeleport))
  (if _result
    (Class|AbilityBase|ConsumeMana)
    (CallFunction|SpawnTeleportParticle)
    (CallFunction|PlaySound))
  (Class|AbilityComponent|EndAbility (Class|AbilityBase|GetAbilityComponent) "Finished"))

(event EventTick
  (params (DeltaSeconds :type Float%20%28single-precision%29))
  (bind _returnvalue (Class|AbilityBase|GetAbilityComponent))
  ;[0 0.272 1] Update effect transform only if ability is pressed but not already casting
  (if (and (Class|AbilityComponent|GetIsPressed _returnvalue) (not (Class|AbilityComponent|GetIsCasting _returnvalue)))
    (CallFunction|UpdateEffect)))

(event EventReleased
  ;[0 0.272 1] On Ability released cast ability or hide spell indicator if not casting
  (bind _returnvalue (Class|AbilityComponent|StartAbility (Class|AbilityBase|GetAbilityComponent)))
  (if _returnvalue
    (Class|AbilityBase|PlayAbilityMontage (Class|AbilityBase|GetAbilityMontage) "None" false 0.0)
    (CallFunction|UpdateEffect)
    (elif (not (Class|AbilityComponent|GetIsCasting (Class|AbilityBase|GetAbilityComponent)))
      (Class|AbilityBase|HideIndicator))))

(event EventPressed
  ;[0 0.272 1] On Ability pressed show spell indicator
  (if (not (Class|AbilityComponent|GetIsCasting (Class|AbilityBase|GetAbilityComponent)))
    (CallFunction|UpdateEffect)
    (Class|AbilityBase|ShowIndicator (Class|AbilityBase|GetEffectLocation))))

(fn ConstructionScript
  (|CallParentFunction))

(fn UpdateEffectTransform
  (bind _returnvalue (Components|GetOwner))
  (bind _returnvalue_2 (Class|AbilityBase|GetEffectLocation))
  (bind _returnvalue_3 (Transformation|GetActorLocation _returnvalue))
  (bind _z (Math|Vector|BreakVector _returnvalue_2))
  ;[0 0.272 1] Calculate Start/End trace location
  (LocalVariables|SetL_TraceStart _returnvalue_3)
  (LocalVariables|SetL_TraceEnd (+ _returnvalue_3 (* (Transformation|GetActorForwardVector (Pawn|GetController (Variables|/Script/Engine.Actor|GetInstigator _returnvalue))) (Variables|Ability|Custom|GetRange))))
  (bind _outhit (Collision|LineTraceForObjects (LocalVariables|GetL_TraceStart) (LocalVariables|GetL_TraceEnd) (Utilities|Array|MakeArray "ObjectTypeQuery1") false 0 "None"))
  (if (.bBlockingHit (Collision|BreakHitResult _outhit))
    (LocalVariables|SetL_HitLocation (.Location (Collision|BreakHitResult _outhit)))
    (if (<= (Class|KismetMathLibrary|DegAcos (Math|Vector|DotProduct (.Normal (Collision|BreakHitResult _outhit)) "0, 0,1.000000")) (Math|Float|Absolute(Float) (Variables|Ability|Custom|GetMaxSurfaceAngle)))
      (LocalVariables|SetL_EffectLocation (LocalVariables|GetL_HitLocation))
      (else
        (LocalVariables|SetL_EffectLocation (Math|Vector|MakeVector (.X (Math|Vector|BreakVector (LocalVariables|GetL_HitLocation))) (.Y (Math|Vector|BreakVector (LocalVariables|GetL_HitLocation))) _z))))
    (else
      (LocalVariables|SetL_EffectLocation (Math|Vector|MakeVector (.X (Math|Vector|BreakVector (LocalVariables|GetL_TraceEnd))) (.Y (Math|Vector|BreakVector (LocalVariables|GetL_TraceEnd))) _z))))
  (return (Math|Transform|MakeTransform (LocalVariables|GetL_EffectLocation) (Transformation|GetActorRotation (Components|GetOwner)))))

(fn AbilityTeleport
  (bind _returnvalue (Components|GetOwner))
  (bind _returnvalue_2 (Transformation|GetActorRotation _returnvalue))
  (bind (_roll _pitch) (Math|Rotator|BreakRotator _returnvalue_2))
  (bind _returnvalue_3 (Transformation|Teleport (Components|GetOwner) (+ (Class|AbilityBase|GetEffectLocation) (Math|Vector|MakeVector 0.0 0.0 (Components|Capsule|GetScaledCapsuleHalfHeight (Variables|/Script/Engine.Character|GetCapsuleComponent (Class|AbilityBase|GetCharacter))))) (Math|Rotator|MakeRotator _roll _pitch (.Yaw (Math|Rotator|BreakRotator (.rotation (Class|AbilityBase|GetEffectTransform)))))))
  (return _returnvalue_3))