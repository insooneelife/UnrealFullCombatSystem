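; Player channeled drain-health ability for the Dynamic Combat System that damages enemies with a beam and heals the owner.
; Pressing retries casting on a timer until it starts or is interrupted; releasing ends it.
; While the effect runs, Tick updates the beam, sphere-traces for attackable pawns and consumes mana.
; Successful hits restore health scaled from damage and attach sparks to the target; ending cleans up particles and sound.
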(event Custom|DrainHealth
  ;[0 0.272 1] Drain health
  (bind _healthcomponent (Variables|Default|GetHealthComponent)
    (:then
      (Class|ExtendedStatComponent|ModifyStat _healthcomponent (* (Class|AbilityBase|GetDamage) (Variables|Ability|Custom|GetDrainScalar)) true))
    (:else)))

(event Custom|UpdateEffect
  ;[0 0.272 1] Update effect
  (Class|AbilityBase|SetEffectTransform (Class|PlayerAbilityBase|GetBeamTransform (Variables|Ability|Custom|GetRange) (Variables|Ability|Custom|GetRadius) (Class|AbilityBase|GetBeamSocket) (Variables|Ability|Custom|GetGoesThroughObjects)))
  (Class|ParticleSystemComponent|SetBeamTargetPoint (Variables|Default|GetBeamParticle) 0 (Class|AbilityBase|GetEffectLocation)))

(event Custom|DestroyBeamParticle
  ;[0 0.272 1] Beam particle events
  (bind _beamparticle (Variables|Default|GetBeamParticle)
    (:then
      (Components|DestroyComponent _beamparticle))
    (:else)))

(event Custom|PlaySound
  ;[0 0.272 1] Sound
  (Variables|Default|GetSoundComponent
    (:then
      _)
    (:else
      (bind _returnvalue (Audio|SpawnSoundAttached (Variables|Ability|Custom|GetSound) (Variables|/Script/Engine.Character|GetMesh (Class|AbilityBase|GetCharacter)) "None" "0, 0, 0" "0, 0, 0" "KeepRelativeOffset" false 1.0 1.0 0.0 0 0))
      (Variables|Default|SetSoundComponent _returnvalue)))
  (Audio|Components|Audio|FadeIn (Variables|Default|GetSoundComponent) 0.5 1.0 0.0 "Linear" :!class /Script/Engine.AudioComponent))

(event Custom|AttempToCastEvent
  ;[0 0.272 1] On Pressed attempt to cast ability until it succeed or gets interrupted
  (CallFunction|AttempttoCast))

(event Custom|ClearAttemptToCastTimer
  ;[0 0.272 1] Clear Attempt To Cast Timer
  (Utilities|Time|ClearTimerbyFunctionName 0 "AttempToCastEvent"))

(event Custom|StopSound
  ;[0 0.272 1] Sound
  (bind _soundcomponent (Variables|Default|GetSoundComponent)
    (:then
      (Audio|Components|Audio|FadeOut _soundcomponent 0.5 0.0 "Linear" :!class /Script/Engine.AudioComponent))
    (:else)))

(event Custom|DeactivateSparksParticle
  ;[0 0.272 1] Sparks particle
  (bind _sparksparticle (Variables|Default|GetSparksParticle)
    (:then
      (Components|Activation|Deactivate _sparksparticle))
    (:else)))

(event Custom|SpawnBeamParticle
  ;[0 0.272 1] Beam particle events
  (bind _returnvalue (Effects|SpawnEmitterAttached (Variables|Ability|Custom|GetDrainBeamParticle) (Variables|/Script/Engine.Character|GetMesh (Class|PlayerAbilityBase|GetPlayerCharacter)) (Class|AbilityBase|GetBeamSocket) "0, 0, 0" "0, 0, 0" "1.000000,1.000000,1.000000" "SnapToTarget"))
  (Variables|Default|SetBeamParticle _returnvalue))

(event Custom|UpdateSparksParticle
  (params (AttachToComponent :type Scene%20Component%20Object%20Reference))
  ;[0 0.272 1] Sparks particle
  (bind _sparksparticle (Variables|Default|GetSparksParticle)
    (:then
      (Components|Activation|Activate _sparksparticle false)
      (if (!= (Transformation|GetAttachParent _sparksparticle) AttachToComponent)
        (Transformation|AttachComponentToComponent (Variables|Default|GetSparksParticle) AttachToComponent "None" "SnapToTarget" "SnapToTarget" "SnapToTarget" true)))
    (:else
      (bind _returnvalue (Effects|SpawnEmitterAttached (Variables|Ability|Custom|GetDrainHitParticle) AttachToComponent "None" "0, 0, 0" "0, 0, 0" "1.000000,1.000000,1.000000" "SnapToTarget"))
      (Variables|Default|SetSparksParticle _returnvalue))))

(event EventInit
  ;[0 0.272 1] Get owner's health component and store in variable
  (Variables|Default|SetHealthComponent (Class|DefaultGameInstance|GetExtendedStatComponent (Components|GetOwner) "Health")))

(event EventPressed
  ;[0 0.272 1] On Pressed attempt to cast ability until it succeed or gets interrupted
  (bind _result (CallFunction|AttempttoCast))
  (if (not _result)
    (Utilities|Time|SetTimerbyEvent (delegate Custom|AttempToCastEvent) 0.1 true)))

(event EventReleased
  ;[0 0.272 1] On released stop ability
  (CallFunction|ClearAttempttoCastTimer)
  (if (Class|AbilityComponent|GetIsCasting (Class|AbilityBase|GetAbilityComponent))
    (Class|AbilityBase|PlayAbilityMontage (Class|AbilityBase|GetAbilityMontage) "End" true 1.0)
    (Class|AbilityComponent|EndAbility (Class|AbilityBase|GetAbilityComponent) "Finished")))

(event EventTick
  (params (DeltaSeconds :type Float%20%28single-precision%29))
  ;[0 0.272 1] Event Tick
  (if (Variables|NonEdit|GetEffectEnabled)
    (CallFunction|UpdateEffect)
    (CallFunction|CheckforEnemies)
    (Class|AbilityBase|ConsumeMana)))

(event EventEnded
  (params (Result :type EAbilityEndResult%20Enum :default "Finished"))
  ;[0 0.272 1] End of ability events
  (CallFunction|ClearAttempttoCastTimer)
  (Variables|NonEdit|SetEffectEnabled false)
  (CallFunction|DestroyBeamParticle)
  (CallFunction|DeactivateSparksParticle)
  (CallFunction|StopSound)
  (switch Utilities|FlowControl|Switch|SwitchonEAbilityEndResult Result
    (:OutOfMana
      (Class|AbilityBase|PlayAbilityMontage (Class|AbilityBase|GetAbilityMontage) "End" true 1.0))))

(event EventEffect
  ;[0 0.272 1] Ability effect
  (Variables|NonEdit|SetEffectEnabled true)
  (CallFunction|SpawnBeamParticle)
  (CallFunction|UpdateEffect)
  (CallFunction|PlaySound))

(fn ConstructionScript
  (|CallParentFunction))

(fn CheckforEnemies
  (bind _returnvalue (Components|GetOwner))
  (bind (_outhit _returnvalue_2) (Collision|SphereTraceForObjects (Transformation|GetSocketLocation (Variables|/Script/Engine.Character|GetMesh (Class|PlayerAbilityBase|GetPlayerCharacter)) (Class|AbilityBase|GetBeamSocket)) (Class|AbilityBase|GetEffectLocation) (Variables|Ability|Custom|GetRadius) (Utilities|Array|MakeArray "ObjectTypeQuery3") false (Utilities|Array|MakeArray (Components|GetOwner)) "None"))
  (if _returnvalue_2
    (if (not (Utilities|Array|ContainsItem (LocalVariables|GetL_HitActors) (.HitActor (Collision|BreakHitResult _outhit))))
      (Utilities|Array|Add (LocalVariables|GetL_HitActors) (.HitActor (Collision|BreakHitResult _outhit)))
      (bind _ascan_be_attacked (Utilities|Casting|CastToCanBeAttacked (.HitActor (Collision|BreakHitResult _outhit))))
      (bind _returnvalue_3 (Class|CanbeAttacked|TakeDamage _ascan_be_attacked (Utilities|Struct|MakeHitData (Class|AbilityBase|GetDamage) _returnvalue (Math|Vector|GetUnitDirection(Vector) (Transformation|GetActorLocation _returnvalue) (Transformation|GetActorLocation (.HitActor (Collision|BreakHitResult _outhit)))) false true false)))
      (if _returnvalue_3
        (CallFunction|DrainHealth)
        (CallFunction|UpdateSparksParticle (.HitComponent (Collision|BreakHitResult _outhit)))))
    (else
      (CallFunction|DeactivateSparksParticle))))

(fn AttempttoCast
  (bind _returnvalue (Class|AbilityComponent|StartAbility (Class|AbilityBase|GetAbilityComponent)))
  (if _returnvalue
    (Class|AbilityBase|PlayAbilityMontage (Class|AbilityBase|GetAbilityMontage) "None" true 1.0)
    (CallFunction|ClearAttempttoCastTimer)
    (return true)
    (else
      (return false))))