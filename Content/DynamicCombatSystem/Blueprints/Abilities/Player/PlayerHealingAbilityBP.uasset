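; Player healing ability in the Dynamic Combat System, channeled to restore health at the cost of mana.
; Pressing retries the cast on a looping timer until it starts the montage, and releasing ends the ability.
; Effect enables per-tick healing and mana consumption, with an attached particle and fading sound.
; Ending stops retries and effects, playing the montage's End section on release or when mana runs out.
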(event Custom|Heal
  ;[0 0.272 1] Heal event
  (bind _healthcomponent (Variables|Default|GetHealthComponent)
    (:then
      (Default|ModifyStat _healthcomponent (Variables|Ability|Custom|GetHealAmount) true))
    (:else)))

(event Custom|SpawnParticle
  ;[0 0.272 1] Particle events
  (bind _particle (Variables|Components|GetParticle)
    (:then
      (Components|Activation|Activate _particle false))
    (:else
      (bind _returnvalue (Effects|SpawnEmitterAttached (Variables|Ability|Custom|GetHealingParticle) (Variables|/Script/Engine.Character|GetMesh (Class|PlayerAbilityBase|GetPlayerCharacter)) "None" "0, 0,100.000000"))
      (Variables|Components|SetParticle _returnvalue))))

(event Custom|DeactivateParticle
  ;[0 0.272 1] Particle events
  (bind _particle (Variables|Components|GetParticle)
    (:then
      (Components|Activation|Deactivate _particle))
    (:else)))

(event Custom|PlaySound
  ;[0 0.272 1] Sound
  (Variables|Default|GetSoundComponent
    (:then
      _)
    (:else
      (bind _returnvalue (Audio|SpawnSoundAttached (Variables|Ability|Custom|GetSound) (Variables|/Script/Engine.Character|GetMesh (Class|AbilityBase|GetCharacter)) "None" "0, 0, 0" "0, 0, 0" "KeepRelativeOffset" false 1.0 1.0 0.0 0 0))
      (Variables|Default|SetSoundComponent _returnvalue)))
  (Audio|Components|Audio|FadeIn (Variables|Default|GetSoundComponent) 0.5 1.0 0.0 "Linear" :!class /Script/Engine.AudioComponent))

(event Custom|AttempToCastEvent
  ;[0 0.272 1] On Pressed attempt to cast ability until it succeed or gets interrupted
  (CallFunction|AttempttoCast))

(event Custom|ClearAttemptToCastTimer
  ;[0 0.272 1] Clear Attempt To Cast Timer
  (Utilities|Time|ClearTimerbyFunctionName 0 "AttempToCastEvent"))

(event Custom|StopSound
  ;[0 0.272 1] Sound
  (bind _soundcomponent (Variables|Default|GetSoundComponent)
    (:then
      (Audio|Components|Audio|FadeOut _soundcomponent 0.5 0.0 "Linear" :!class /Script/Engine.AudioComponent))
    (:else)))

(event EventInit
  ;[0 0.272 1] Get owner's health component and store in variable
  (Variables|Default|SetHealthComponent (CallFunction|GetExtendedStatComponent (Components|GetOwner) "NewEnumerator1")))

(event EventEffect
  ;[0 0.272 1] Ability effect
  (Variables|NonEdit|SetEffectEnabled true)
  (CallFunction|SpawnParticle)
  (CallFunction|PlaySound))

(event EventEnded
  (params (Result :type EAbilityEndResult%20Enum :default "Finished"))
  ;[0 0.272 1] End of ability events
  (CallFunction|ClearAttempttoCastTimer)
  (Variables|NonEdit|SetEffectEnabled false)
  (CallFunction|DeactivateParticle)
  (CallFunction|StopSound)
  (switch Utilities|FlowControl|Switch|SwitchonEAbilityEndResult Result
    (:OutOfMana
      (Class|AbilityBase|PlayAbilityMontage (Class|AbilityBase|GetAbilityMontage) "End" true 1.0))))

(event EventReleased
  ;[0 0.272 1] On released stop ability
  (CallFunction|ClearAttempttoCastTimer)
  (if (Class|AbilityComponent|GetIsCasting (Class|AbilityBase|GetAbilityComponent))
    (Class|AbilityBase|PlayAbilityMontage (Class|AbilityBase|GetAbilityMontage) "End" true 1.0)
    (Class|AbilityComponent|EndAbility (Class|AbilityBase|GetAbilityComponent) "Finished")))

(event EventPressed
  ;[0 0.272 1] On Pressed attempt to cast ability until it succeed or gets interrupted
  (bind _result (CallFunction|AttempttoCast))
  (if (not _result)
    (Utilities|Time|SetTimerbyEvent (delegate Custom|AttempToCastEvent) 0.1 true)))

(event EventTick
  (params (DeltaSeconds :type Float%20%28single-precision%29))
  ;[0 0.272 1] Keep healing and consuming mana while effect is enabled
  (if (Variables|NonEdit|GetEffectEnabled)
    (CallFunction|Heal)
    (Class|AbilityBase|ConsumeMana)))

(fn ConstructionScript)

(fn AttempttoCast
  (bind _returnvalue (Class|AbilityComponent|StartAbility (Class|AbilityBase|GetAbilityComponent)))
  (if _returnvalue
    (Class|AbilityBase|PlayAbilityMontage (Class|AbilityBase|GetAbilityMontage) "None" true 1.0)
    (CallFunction|ClearAttempttoCastTimer)
    (return true)
    (else
      (return false))))