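; Anim notify state in the Dynamic Combat System that marks a chosen activity as active on the owning actor for the span of an animation window.
; On begin it finds the owner's StateManagerComponentBP and sets the Activity to true, and on end sets it back to false, doing nothing if either is missing.
; The notify's timeline label shows the selected Activity enum's name.
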(fn ReceivedNotifyBegin
  (params (MeshComp :type Skeletal%20Mesh%20Component%20Object%20Reference) (Animation :type Anim%20Sequence%20Base%20Object%20Reference) (TotalDuration :type Float%20%28single-precision%29))
  (bind _returnvalue (Components|GetOwner MeshComp))
  (bind _returnvalue_2 (Actor|GetComponentbyClass _returnvalue "/Game/DynamicCombatSystem/Blueprints/Components/StateManagerComponentBP.StateManagerComponentBP_C"))
  (Utilities|IsValid _returnvalue
    (:Is%20Valid
      (Utilities|IsValid _returnvalue_2
        (:Is%20Valid
          (Default|SetActivity _returnvalue_2 (Variables|Default|GetActivity) true)
          (return false))))))

(fn ReceivedNotifyEnd
  (params (MeshComp :type Skeletal%20Mesh%20Component%20Object%20Reference) (Animation :type Anim%20Sequence%20Base%20Object%20Reference))
  (bind _returnvalue (Components|GetOwner MeshComp))
  (bind _returnvalue_2 (Actor|GetComponentbyClass _returnvalue "/Game/DynamicCombatSystem/Blueprints/Components/StateManagerComponentBP.StateManagerComponentBP_C"))
  (Utilities|IsValid _returnvalue
    (:Is%20Valid
      (Utilities|IsValid _returnvalue_2
        (:Is%20Valid
          (Default|SetActivity _returnvalue_2 (Variables|Default|GetActivity) false)
          (return false))))))

(fn GetNotifyName
  (return (Utilities|String|EnumtoString (Variables|Default|GetActivity))))