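; Anim notify that shows or hides the arrow on the owner's bow and sets whether it attaches to the hand or the bow during an animation.
; It gets the owner's EquipmentComponent, casts the displayed RangeWeapon item in slot 0 to BowDisplayedItem, then updates arrow attachment and visibility from its Visible and AttachToHand settings.
; The notify name is built from those settings, so it describes the configured action.
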(fn ReceivedNotify
  (params (MeshComp :type Skeletal%20Mesh%20Component%20Object%20Reference) (Animation :type Anim%20Sequence%20Base%20Object%20Reference))
  (bind _returnvalue (Components|GetOwner MeshComp))
  (bind _returnvalue_2 (Actor|GetComponentbyClass _returnvalue "/Script/DynamicCombatFull.EquipmentComponent"))
  (bind _returnvalue_3 (Class|EquipmentComponent|GetDisplayedItem _returnvalue_2 "RangeWeapon"))
  (Utilities|IsValid _returnvalue
    (:Is%20Valid
      (Utilities|IsValid _returnvalue_2
        (:Is%20Valid
          (Utilities|IsValid _returnvalue_3
            (:Is%20Valid
              (bind _asbow_displayed_item (Utilities|Casting|CastToBowDisplayedItem _returnvalue_3))
              (Class|BowDisplayedItem|UpdateArrowAttachment _asbow_displayed_item (Variables|Default|GetAttachToHand))
              (Class|BowDisplayedItem|UpdateArrowVisibility _asbow_displayed_item (Variables|Default|GetVisible))
              (return false))))))))

(fn GetNotifyName
  (return (Utilities|String|Append (select (Variables|Default|GetVisible) "Show" "Hide") " Arrow" (select (Variables|Default|GetVisible) (Utilities|String|Append " and attach to " (select (Variables|Default|GetAttachToHand) "Hand" "Bow")) ""))))