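; HitBox anim notify state that opens and closes an actor's hit detection window during an animation in the Dynamic Combat System.
; On begin, it finds the owner's CollisionHandlerComponent and activates collision for the configured CollisionPart.
; On end, it deactivates collision on that component.
; Both events return false when the owner has no valid component.
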(fn ReceivedNotifyEnd
  (params (MeshComp :type Skeletal%20Mesh%20Component%20Object%20Reference) (Animation :type Anim%20Sequence%20Base%20Object%20Reference))
  (bind _returnvalue (Components|GetOwner MeshComp))
  (bind _returnvalue_2 (Actor|GetComponentbyClass _returnvalue "/Script/DynamicCombatFull.CollisionHandlerComponent"))
  (Utilities|IsValid _returnvalue_2
    (:Is%20Valid
      (Class|CollisionHandlerComponent|DeactivateCollision _returnvalue_2)
      (return true))
    (:Is%20Not%20Valid
      (return false))))

(fn GetNotifyName
  (return "HitBox"))

(fn ReceivedNotifyBegin
  (params (MeshComp :type Skeletal%20Mesh%20Component%20Object%20Reference) (Animation :type Anim%20Sequence%20Base%20Object%20Reference) (TotalDuration :type Float%20%28single-precision%29))
  (bind _returnvalue (Components|GetOwner MeshComp))
  (bind _returnvalue_2 (Actor|GetComponentbyClass _returnvalue "/Script/DynamicCombatFull.CollisionHandlerComponent"))
  (Utilities|IsValid _returnvalue_2
    (:Is%20Valid
      (Class|CollisionHandlerComponent|ActivateCollision _returnvalue_2 (Variables|Default|GetCollisionPart))
      (return true))
    (:Is%20Not%20Valid
      (return false))))