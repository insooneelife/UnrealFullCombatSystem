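; Anim notify in the Dynamic Combat System that applies backstab damage to the mesh's owner at a point in an animation.
; It checks the owner's effects component for a specific effect, taking the damage amount from that component and crediting the effect's applier.
; The hit goes through TakeDamageMessage as unblockable and without impact, and a hit sound plays at the owner's location on success.
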(fn ReceivedNotify
  (params (MeshComp :type Skeletal%20Mesh%20Component%20Object%20Reference) (Animation :type Anim%20Sequence%20Base%20Object%20Reference))
  (bind _returnvalue (Components|GetOwner MeshComp))
  (bind _returnvalue_2 (Components|GetOwner MeshComp))
  (Utilities|IsValid _returnvalue
    (:Is%20Valid
      (LocalVariables|SetL_EffectsComponent (Actor|GetComponentbyClass _returnvalue "/Game/DynamicCombatSystem/Blueprints/Components/EffectsComponentBP.EffectsComponentBP_C"))
      (bind _l_effectscomponent (LocalVariables|GetL_EffectsComponent)
        (:then
          (if (Default|IsEffectApplied _l_effectscomponent "NewEnumerator7")
            (bind _result (Class|ICanbeAttacked|TakeDamage(Message) (Components|GetOwner MeshComp) (Utilities|Struct|MakeF_HitData (Variables|/Game/DynamicCombatSystem/Blueprints/Components/EffectsComponentBP.EffectsComponentBP_C|GetBackstabDamage (LocalVariables|GetL_EffectsComponent)) (Default|GetEffectApplier (LocalVariables|GetL_EffectsComponent) "NewEnumerator7") "0.000000,0.000000,0.000000" false false false)))
            (if _result
              (CallFunction|PlayHitSound (Default|GetEffectApplier (LocalVariables|GetL_EffectsComponent) "NewEnumerator7") _returnvalue_2 (Transformation|GetActorLocation _returnvalue_2))
              (return false))))
        (:else)))))

(fn GetNotifyName
  (return "GetBackstabDmg"))