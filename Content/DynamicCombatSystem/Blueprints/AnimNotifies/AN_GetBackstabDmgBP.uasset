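; Anim notify in the Dynamic Combat System that deals backstab damage to the mesh owner at a timed point in an animation.
; It acts only while the owner's EffectsComponent has the Backstab effect, taking the damage amount and effect applier from that component.
; The unblockable, impact-free hit goes through the CanBeAttacked interface, and a successful TakeDamage plays the hit sound at the owner's location.
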(fn ReceivedNotify
  (params (MeshComp :type Skeletal%20Mesh%20Component%20Object%20Reference) (Animation :type Anim%20Sequence%20Base%20Object%20Reference))
  (bind _returnvalue (Components|GetOwner MeshComp))
  (bind _returnvalue_2 (Components|GetOwner MeshComp))
  (Utilities|IsValid _returnvalue
    (:Is%20Valid
      (bind _output_get (LocalVariables|SetL_EffectsComponent (Actor|GetComponentbyClass _returnvalue "/Script/DynamicCombatFull.EffectsComponent")))
      (Utilities|IsValid _output_get
        (:Is%20Valid
          (if (Class|EffectsComponent|IsEffectApplied _output_get "Backstab")
            (bind _ascan_be_attacked (Utilities|Casting|CastToCanBeAttacked (Components|GetOwner MeshComp)))
            (bind _returnvalue_3 (Class|CanbeAttacked|TakeDamage _ascan_be_attacked (Utilities|Struct|MakeHitData (Class|EffectsComponent|GetBackstabDamage (LocalVariables|GetL_EffectsComponent)) (Class|EffectsComponent|GetEffectApplier (LocalVariables|GetL_EffectsComponent) "Backstab") "0.000000,0.000000,0.000000" false false false)))
            (if _returnvalue_3
              (CallFunction|PlayHitSound (Class|EffectsComponent|GetEffectApplier (LocalVariables|GetL_EffectsComponent) "Backstab") _returnvalue_2 (Transformation|GetActorLocation _returnvalue_2))
              (return false))))))))

(fn GetNotifyName
  (return "GetBackstabDmg"))