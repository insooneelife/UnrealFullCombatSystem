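; Anim notify state "HitBox" that opens a melee-style collision window during an animation in the Dynamic Combat System.
; On begin it finds the owner's CollisionHandlerComponentBP and activates collision for the configured CollisionPart.
; On end it deactivates collision on that component, and both events return false when the owner lacks a valid component.
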(fn ReceivedNotifyEnd
  (params (MeshComp :type Skeletal%20Mesh%20Component%20Object%20Reference) (Animation :type Anim%20Sequence%20Base%20Object%20Reference))
  (bind _returnvalue (Components|GetOwner MeshComp))
  (bind _returnvalue_2 (Actor|GetComponentbyClass _returnvalue "/Game/DynamicCombatSystem/Blueprints/Components/CollisionHandlerComponentBP.CollisionHandlerComponentBP_C"))
  (Utilities|IsValid _returnvalue_2
    (:Is%20Valid
      (Default|DeactivateCollision _returnvalue_2)
      (return true))
    (:Is%20Not%20Valid
      (return false))))

(fn GetNotifyName
  (return "HitBox"))

(fn ReceivedNotifyBegin
  (params (MeshComp :type Skeletal%20Mesh%20Component%20Object%20Reference) (Animation :type Anim%20Sequence%20Base%20Object%20Reference) (TotalDuration :type Float%20%28single-precision%29))
  (bind _returnvalue (Components|GetOwner MeshComp))
  (bind _returnvalue_2 (Actor|GetComponentbyClass _returnvalue "/Game/DynamicCombatSystem/Blueprints/Components/CollisionHandlerComponentBP.CollisionHandlerComponentBP_C"))
  (Utilities|IsValid _returnvalue_2
    (:Is%20Valid
      (Default|ActivateCollision _returnvalue_2 (Variables|Default|GetCollisionPart))
      (return true))
    (:Is%20Not%20Valid
      (return false))))