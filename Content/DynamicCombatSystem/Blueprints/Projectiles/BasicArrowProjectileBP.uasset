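; Basic arrow projectile in the Dynamic Combat System that can leave an impaled arrow in what it hits.
; SpawnImpaledArrow halts projectile movement and spawns BP_ImpaledArrow at the given location, copying the arrow's rotation, scale and mesh.
; The new arrow is owned by the given actor and attached to the given component socket, keeping its world transform.
; Hit detection and the event's caller lie outside this graph.
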(event EventBeginPlay)

(event Collision|EventActorBeginOverlap
  (params (OtherActor :type Actor%20Object%20Reference)))

(event EventTick
  (params (DeltaSeconds :type Float%20%28single-precision%29)))

(event EventSpawnImpaledArrow
  (params (InComponent :type Scene%20Component%20Object%20Reference) (InSocketName :type Name :default "None") (InActor :type Actor%20Object%20Reference) (InLocation :type Vector :default "0, 0, 0"))
  (Components|Movement|StopMovementImmediately (Variables|Default|GetProjectileMovement))
  (bind _returnvalue (Game|SpawnActorfromClass "/Game/DynamicCombatSystem/Blueprints/Projectiles/BP_ImpaledArrow.BP_ImpaledArrow_C" (Math|Transform|MakeTransform InLocation (Transformation|GetActorRotation) (Transformation|GetActorScale3D)) "AlwaysSpawn" InActor (Variables|/Script/Engine.StaticMeshComponent|GetStaticMesh (Variables|Default|GetStaticMesh)) (Game|GetInstigator (Components|GetOwner))))
  (Transformation|AttachComponentToComponent _returnvalue InComponent InSocketName "KeepWorld" "KeepWorld" "KeepWorld" true))

(fn ConstructionScript)